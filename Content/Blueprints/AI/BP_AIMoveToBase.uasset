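; BP_AIMoveToBase is an AI helper whose FindNearestActorOfClass function finds the nearest intact BP_TheWall to a target location.
; It loops over every wall, flags and skips those marked Destroy, and keeps the closest of the rest by distance.
; It returns that distance, the wall and whether any destroyed wall was found.
; The Class input is ignored because the wall class is hardcoded.
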(fn FindNearestActorOfClass
  (params (Class :type Actor%20Object%20Reference) (TargetLocation :type Vector))
  (bind _outactors (Actor|GetAllActorsOfClass 0 "/Game/Blueprints/BP_TheWall.BP_TheWall_C"))
  (for _array_element _outactors
    (if (Variables|/Game/Blueprints/BP_TheWall.BP_TheWall_C|GetDestroy _array_element)
      (LocalVariables|SetDestroyedWallFound true)
      (elif (< (Math|Vector|Distance(Vector) (Transformation|GetActorLocation _array_element) TargetLocation) (LocalVariables|GetNewLocalVar_0))
        (LocalVariables|SetNewLocalVar_0 (Math|Vector|Distance(Vector) (Transformation|GetActorLocation _array_element) TargetLocation))
        (LocalVariables|SetNewLocalVar_1 _array_element))))
  (return (LocalVariables|GetNewLocalVar_0) (LocalVariables|GetNewLocalVar_1) (LocalVariables|GetDestroyedWallFound)))